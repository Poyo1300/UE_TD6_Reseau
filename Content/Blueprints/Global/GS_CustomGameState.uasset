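; GS_CustomGameState is a game state Blueprint that runs the match countdown.
; On BeginPlay it copies GameTime from GI_CustomGameInstance, and only the server starts a looping one-second timer.
; Each tick decrements GameTime and passes it to the HUD widget of player controller 0, cast to PC_CustomPlayerController.
; The graph has no handling for the countdown reaching zero.
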(event `self.ReceiveBeginPlay`
  (set `self.GameTime` (`CustomGameInstance.GameTime` (cast `/Game/Blueprints/Global/GI_CustomGameInstance` (`GameplayStatics.GetGameInstance`) :!pure true)))
  (if (`KismetSystemLibrary.IsServer`)
    (`KismetSystemLibrary.K2_SetTimerDelegate` (delegate `Update Timer`) 1.0 true)))

(event `Update Timer`
  (bind _output_get (set `self.GameTime` (- (`self.GameTime`) 1)))
  (`/Game/Blueprints/Widget/WBP_HUD.Update Timer` (`/Game/Blueprints/Player/PC_CustomPlayerController.HUDWidget` (cast `/Game/Blueprints/Player/PC_CustomPlayerController` (`GameplayStatics.GetPlayerController` 0) :!pure true)) _output_get))

(fn `UserConstructionScript`)