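; GM_Menu is the menu game mode that fills the lobby browser with online sessions found by a session search.
; On BeginPlay it binds to the session subsystem's find-completed event, then stores successful results and passes each to AddLobby.
; AddLobby creates a WBP_LobbyInfos widget per session and appends it to the WBP_LobbyWindow list.
; A RemoveOldLobby event clears that list.
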(event `self.ReceiveBeginPlay`
  (add `OnlineSessionSubsystem.OnFindSessionsCompletedEvent` (subsystem `OnlineSessionSubsystem`) (delegate `OnFindSessions`)))

(event `OnFindSessions`
  (params (SessionResult :type "Array of SessionInfo Structure (by ref)") (bSuccessful :type Boolean))
  (if bSuccessful
    (bind _output_get (set `self.Session Result` SessionResult))
    (for _array_element _output_get
      (`self.AddLobby` _array_element))))

(event `self.RemoveOldLobby`
  (bind _aswbp_lobby_window (cast `/Game/Blueprints/Widget/WBP_LobbyWindow` (`self.LobbyWindowWidget`)))
  (`/Game/Blueprints/Widget/WBP_LobbyWindow.ClearLobbyList` _aswbp_lobby_window))

(fn `AddLobby`
  (params (Infos :type "SessionInfo Structure"))
  (bind _returnvalue (`|CreateWidget` "/Game/Blueprints/Widget/WBP_LobbyInfos.WBP_LobbyInfos_C" (`GameplayStatics.GetPlayerController` 0) Infos))
  (bind _aswbp_lobby_window (cast `/Game/Blueprints/Widget/WBP_LobbyWindow` (`self.LobbyWindowWidget`)))
  (`/Game/Blueprints/Widget/WBP_LobbyWindow.AddLobbyToList` _aswbp_lobby_window _returnvalue))

(fn `UserConstructionScript`)