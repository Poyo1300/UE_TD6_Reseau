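; Lobby game mode that opens a host beacon for online sessions and keeps the lobby's player list current.
; On BeginPlay it creates the beacon through the online session subsystem on a fixed listen port.
; UpdatePlayer waits briefly, rebuilds GS_LobbyGameState's PlayersState from PlayerArray entries that cast to BP_CustomPlayerState, then has the game state update teams.
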(event `self.ReceiveBeginPlay`
  (`OnlineSessionSubsystem.CreateHostBeacon` (subsystem `OnlineSessionSubsystem`) 19250 false))

(event `self.UpdatePlayer`
  (params (Controller :type "Controller Object Reference"))
  (bind _asgs_lobby_game_state (cast `/Game/Blueprints/Global/GS_LobbyGameState` (`GameplayStatics.GetGameState`) :!pure true))
  (bind _playersstate (`/Game/Blueprints/Global/GS_LobbyGameState.PlayersState` _asgs_lobby_game_state))
  (`KismetSystemLibrary.Delay` 0.1)
  (`KismetArrayLibrary.Array_Clear` _playersstate)
  (for _array_element (`GameStateBase.PlayerArray` _asgs_lobby_game_state)
    (bind _asbp_custom_player_state (cast `/Game/Blueprints/Player/BP_CustomPlayerState` _array_element))
    (`KismetArrayLibrary.Array_Add` _playersstate _asbp_custom_player_state))
  (`/Game/Blueprints/Global/GS_LobbyGameState.UpdateTeams` _asgs_lobby_game_state))

(fn `UserConstructionScript`)