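; PC_CustomPlayerController is the player controller that creates the HUD and initializes the player's lives display.
; On BeginPlay, the local controller adds WBP_HUD to the viewport, sets game-only input and hides the cursor.
; After a short delay, it copies MaxLives from GI_CustomGameInstance to BP_CustomCharacter.
; An UpdatePlayerLives event forwards lives values to the HUD, including that initial value.
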(event `self.ReceiveBeginPlay`
  (bind _maxlives (`CustomGameInstance.MaxLives` (cast `/Game/Blueprints/Global/GI_CustomGameInstance` (`GameplayStatics.GetGameInstance`) :!pure true)))
  (if (`self.IsLocalController`)
    (bind _returnvalue (`|CreateWidget` "/Game/Blueprints/Widget/WBP_HUD.WBP_HUD_C"))
    (bind _output_get (set `self.HUDWidget` _returnvalue))
    (`UserWidget.AddToViewport` _output_get 0)
    (`WidgetBlueprintLibrary.SetInputMode_GameOnly` self)
    (set `self.bShowMouseCursor` false)
    (`KismetSystemLibrary.Delay` 0.02)
    (set `CustomCharacter.Lives` _maxlives (cast `/Game/Blueprints/Player/BP_CustomCharacter` (`GameplayStatics.GetPlayerCharacter` 0) :!pure true))
    (`self.UpdatePlayerLives` _maxlives)))

(event `self.UpdatePlayerLives`
  (params (Value :type Integer))
  (`/Game/Blueprints/Widget/WBP_HUD.Update Lives` (`self.HUDWidget`) Value))

(fn `UserConstructionScript`)